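; BP_StoredFood is the actor for a food item placed in a storage zone, showing its mesh and remaining expiry.
; BeginPlay plays a sound, caches the StoringPawn and copies its current FoodData to set the mesh.
; SpawnOnShelf positions and scales it at hardcoded coordinates, diverting high placements to door shelves whose height comes from the pawn's zone.
; Expiry appears as color-coded text dashes; an older widget version and an unused Z-adjustment helper remain.
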(event `self.ReceiveBeginPlay`
  (`GameplayStatics.PlaySoundAtLocation` "/Game/LevelsParameters/Storing/SFX/StoredObject.StoredObject" (`self.K2_GetActorLocation` self) (struct) 1.0 1.0 0.0 null null null null)
  ;[1 1 1] Getting a reference to storingPawn to avoid recasts
  (`/Engine/EditorBlueprintResources/StandardMacros.IsValid` (`self.PawnRef`)
    (:`Is Not Valid`
      (bind _asstoring_pawn (cast `/Game/LevelsParameters/Storing/StoringPawn` (`GameplayStatics.GetPlayerPawn` 0))
        (:`then`
          (set `self.PawnRef` _asstoring_pawn)
          (set `self.FoodData` (`/Game/LevelsParameters/Storing/BP_SelectFood.FoodData` (`/Game/LevelsParameters/Storing/StoringPawn.FoodRef` (`self.PawnRef`))))
          (`StaticMeshComponent.SetStaticMesh` (`self.StaticMesh`) (`/Game/LevelsParameters/Storing/Structures/FoodDataAsset.Mesh` (`self.FoodData`))))
        (:`CastFailed`
          (`KismetSystemLibrary.PrintString` "you trolling you have no storing pawn"))))))

(event `self.ReceiveActorBeginOverlap`
  (params (OtherActor :type "Actor Object Reference")))

(event `self.ReceiveTick`
  (params (DeltaSeconds :type "Float (single-precision)")))

(fn `ChangeExpiryProgressNEW`
  (locals (Red :type "Color Structure" :default (struct :`R` 250 :`A` 255)) (Orange :type "Color Structure" :default (struct :`G` 89 :`R` 255 :`A` 255)) (Yellow :type "Color Structure" :default (struct :`B` 11 :`G` 196 :`R` 229 :`A` 255)) (YellowGreen :type "Color Structure" :default (struct :`B` 13 :`G` 141 :`R` 112 :`A` 255)) (Green :type "Color Structure" :default (struct :`G` 139 :`R` 39 :`A` 255)))
  (bind _expirydots (`self.ExpiryDots`))
  (switch `int` (`self.ExpiryPeriod`)
    (:`0`
      (`TextRenderComponent.SetTextRenderColor` :`self` _expirydots))
    (:`1`
      (`TextRenderComponent.SetTextRenderColor` _expirydots (`local.Red`))
      (set `self.ExpiryText` "- "))
    (:`2`
      (`TextRenderComponent.SetTextRenderColor` _expirydots (`local.Orange`))
      (set `self.ExpiryText` "- -"))
    (:`3`
      (`TextRenderComponent.SetTextRenderColor` _expirydots (`local.Yellow`))
      (set `self.ExpiryText` "- - -"))
    (:`4`
      (`TextRenderComponent.SetTextRenderColor` _expirydots (`local.Green`))
      (set `self.ExpiryText` "- - - -")))
  (`TextRenderComponent.K2_SetText` _expirydots (`self.ExpiryText`)))

(fn `ChangeExpiryProgressOLD`
  (bind _aswbp_expiry (cast `/Game/UIElements/WBP_Expiry` (`WidgetComponent.GetWidget` (`self.ExpiryProgressBar`))))
  (set `/Game/UIElements/WBP_Expiry.ExpiryDate` (`self.ExpiryPeriod`) _aswbp_expiry))

(fn `SpawnOnDoor`
  (locals (ZAxisAdjust :type "Float (double-precision)"))
  (bind _currentzonerefcopy (`/Game/LevelsParameters/Storing/StoringPawn.CurrentZoneRefCopy` (`self.PawnRef`)))
  (bind _ztransform (`/Game/LevelsParameters/Storing/BP_StoringZone.StoreDoorShelves` _currentzonerefcopy (`/Game/LevelsParameters/Storing/BP_StoringZone.Capacity` _currentzonerefcopy)))
  (bind (_returnvalue_location _returnvalue_rotation _returnvalue_scale) (`KismetMathLibrary.BreakTransform` (`KismetMathLibrary.MakeTransform` (`KismetMathLibrary.MakeVector` 938.0 -158.548499 _ztransform) (struct) (`KismetMathLibrary.Conv_DoubleToVector` (`/Game/LevelsParameters/Storing/Structures/FoodDataAsset.TransformScaleMultiply` (`self.FoodData`))))))
  (`self.K2_SetActorTransform` (`KismetMathLibrary.MakeTransform` _returnvalue_location))
  (`SceneComponent.SetWorldScale3D` (`self.StaticMesh`) _returnvalue_scale))

(fn `SpawnOnShelf`
  (params (ZTransform :type "Float (double-precision)") (YTransform :type "Float (double-precision)"))
  (locals (ZAxisAdjust :type "Float (double-precision)"))
  (bind (_returnvalue_location _returnvalue_rotation _returnvalue_scale) (`KismetMathLibrary.BreakTransform` (`KismetMathLibrary.MakeTransform` (`KismetMathLibrary.MakeVector` 954.0 YTransform (- ZTransform 23.0)) (struct) (`KismetMathLibrary.Conv_DoubleToVector` (`/Game/LevelsParameters/Storing/Structures/FoodDataAsset.TransformScaleMultiply` (`self.FoodData`))))))
  (if (> ZTransform 510.0)
    (`self.SpawnOnDoor`)
    (else
      (`self.K2_SetActorTransform` (`KismetMathLibrary.MakeTransform` _returnvalue_location))
      (`SceneComponent.SetWorldScale3D` (`self.StaticMesh`) _returnvalue_scale))))

(fn `UserConstructionScript`
  (`AddComponent|NODE_AddNiagaraComponent-0`))

(fn `ZAxisAdjustmentUNUSED`
  (returns (ReturnValue :type "Float (double-precision)"))
  (locals (ZAdjustment :type "Float (double-precision)"))
  ;[1 1 1] Tentar fazer com o nome da prateleira em si?
  (switch `int` 0
    (:`1`
      ;[1 1 1] Pantry
      (set `local.ZAdjustment` 23.0))
    (:`2`
      ;[1 1 1] Fridge
      (set `local.ZAdjustment` 23.0))
    (:`3`
      ;[1 1 1] Freezer
      (set `local.ZAdjustment` 23.0)))
  (return (`local.ZAdjustment`)))