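; Touch-selectable food item for the food-storing level, taking its mesh from FoodData and bobbing up and down on a looping timer started after a random delay.
; Touching it stops its bob, resumes the bob on all other food items and passes itself and its mesh to the StoringPawn.
; ThrowFood enables physics and applies an impulse chosen by the storing zone's display name to toss it toward that fridge, freezer or pantry spot.
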(event `self.ReceiveBeginPlay`
  ;[1 1 1] Getting a reference to storingPawn to avoid recasts
  (`/Engine/EditorBlueprintResources/StandardMacros.IsValid` (`self.PawnRef`)
    (:`Is Not Valid`
      (bind _asstoring_pawn (cast `/Game/LevelsParameters/Storing/StoringPawn` (`GameplayStatics.GetPlayerPawn` 0))
        (:`then`
          (set `self.PawnRef` _asstoring_pawn)
          (`self.StartJump`))
        (:`CastFailed`
          (`KismetSystemLibrary.PrintString` "you trolling you have no storing pawn"))))))

(event `StartJump`
  (`KismetSystemLibrary.Delay` (`KismetMathLibrary.RandomFloatInRange` 0.0 1.0))
  (`KismetSystemLibrary.K2_SetTimerDelegate` (delegate `MoveFood`) 0.02 true) ; First time
)

(event `self.ReceiveActorBeginOverlap`
  (params (OtherActor :type "Actor Object Reference")))

(event `self.ReceiveTick`
  (params (DeltaSeconds :type "Float (single-precision)")))

(event `MoveFood`
  (if (not (`self.StopJump`))
    (`self.FoodJump`)))

(event `self.StaticMesh.OnInputTouchBegin`
  (params (FingerIndex :type "ETouchIndex Enum" :default "Touch1") (TouchedComponent :type "PrimitiveComponent Object Reference"))
  (bind _pawnref (`self.PawnRef`))
  (`GameplayStatics.PlaySound2D` "/Game/LevelsParameters/InteractFood2.InteractFood2" 1.0 1.0 0.0 null null)
  (bind _outactors (`GameplayStatics.GetAllActorsOfClass` "BP_SelectFood_C"))
  (for _array_element _outactors
    (if (not (== _array_element self))
      (set `/Game/LevelsParameters/Storing/BP_SelectFood.StopJump` false _array_element)))
  (`/Game/LevelsParameters/Storing/StoringPawn.SetFoodRef` _pawnref self)
  (`/Game/LevelsParameters/Storing/StoringPawn.ChangeFoodMesh (Changed)` _pawnref (`StaticMeshComponent.StaticMesh` (`self.StaticMesh`)))
  (set `self.StopJump` true))

(fn `DisableSimulatePhysics`
  (`PrimitiveComponent.SetSimulatePhysics` (`self.StaticMesh`) false))

(fn `FoodJump`
  (locals (ZMax :type "Float (double-precision)" :default 28.0) (ZMin :type "Float (double-precision)" :default 8.0))
  (bind _defaultsceneroot (`self.DefaultSceneRoot`))
  (bind _currentzposition (`self.CurrentZPosition`))
  (bind _returnvalue (`SceneComponent.GetRelativeTransform` _defaultsceneroot))
  (if (`self.isMovUp`)
    (if (== (`local.ZMax`) _currentzposition)
      (set `self.isMovUp` false)
      (else
        (`/Engine/EditorBlueprintResources/StandardMacros.IncrementFloat` _currentzposition
          (:`  `
            (`SceneComponent.K2_SetRelativeLocation` _defaultsceneroot (`KismetMathLibrary.MakeVector` (.x (.location _returnvalue)) (.y (.location _returnvalue)) _currentzposition) false false :!label _label)))))
    (elif (== (`local.ZMin`) _currentzposition)
      (set `self.isMovUp` true)
      (else
        (`/Engine/EditorBlueprintResources/StandardMacros.DecrementFloat` _currentzposition
          (:`  `
            (goto _label)))))))

(fn `ThrowFood`
  (params (StoringZone :type "/Game/LevelsParameters/Storing/BP_StoringZone Object Reference"))
  (bind _staticmesh (`self.StaticMesh`))
  (`PrimitiveComponent.SetSimulatePhysics` _staticmesh true)
  (switch `string` (`KismetSystemLibrary.GetDisplayName` StoringZone)
    (:`FridgeShelf1`
      ;[1 1 1] Fridge Shelf 1 & Pantry Shelf 1
      (`PrimitiveComponent.AddImpulse` _staticmesh (300.0 0.0 200.0) "None" false :!label _label))
    (:`PantryShelf1`
      (goto _label))
    (:`FridgeShelf2`
      ;[1 1 1] Fridge Shelf 2 & Freezer 1
      (`PrimitiveComponent.AddImpulse` _staticmesh (300.0 0.0 110.0) "None" false :!label _label_2))
    (:`PantryShelf2`
      (`PrimitiveComponent.AddImpulse` _staticmesh (300.0 0.0 50.0) "None" false))
    (:`FridgeShelf3`
      ;[1 1 1] Fridge Shelf 3 & Pantry Shelf 2 & Freezer 2
      (`PrimitiveComponent.AddImpulse` _staticmesh (300.0 0.0 23.0) "None" false :!label _label_3))
    (:`PantryShelf3`
      ;[1 1 1] Fridge Shelf 4 & Pantry Shelf 3 & Freezer 3
      (`PrimitiveComponent.AddImpulse` _staticmesh (300.0 0.0 -50.0) "None" false :!label _label_4))
    (:`FridgeShelf4`
      (goto _label_4))
    (:`FreezerShelf1`
      (goto _label_2))
    (:`FreezerShelf2`
      (goto _label_3))
    (:`FreezerShelf3`
      (goto _label_4))
    (:`FridgeDoor`
      ;[1 1 1] Fridge Left door
      (`PrimitiveComponent.AddImpulse` _staticmesh (300.0 -180.0 0.0) "None" false))))

(fn `UserConstructionScript`
  (`StaticMeshComponent.SetStaticMesh` (`self.StaticMesh`) (`/Game/LevelsParameters/Storing/Structures/FoodDataAsset.Mesh` (`self.FoodData`))))