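; Touchable zone selector for the food-storing level that moves the StoringPawn between an overview and pantry, fridge or freezer close-ups.
; ZoneMesh touches check pawn position before zooming and show Portuguese/English hints, while Sphere touches call ZoomLocation directly.
; ZoomLocation spawns a BP_StoringArrow and toggles labels and zone overlays, with its default case restoring the overview.
; On Day1 it also reveals example food meshes and swipe clues.
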(event `self.ReceiveBeginPlay`
  ;[1 1 1] Getting a reference to storingPawn to avoid recasts
  (`/Engine/EditorBlueprintResources/StandardMacros.IsValid` (`self.PawnRef`)
    (:`Is Not Valid`
      (bind _asstoring_pawn (cast `/Game/LevelsParameters/Storing/StoringPawn` (`GameplayStatics.GetPlayerPawn` 0))
        (:`then`
          (set `self.PawnRef` _asstoring_pawn)
          (set `self.MaterialRef` (`self.Material`)))
        (:`CastFailed`
          (`KismetSystemLibrary.PrintString` "you trolling you have no storing pawn"))))))

(event `self.ReceiveActorBeginOverlap`
  (params (OtherActor :type "Actor Object Reference")))

(event `self.ReceiveTick`
  (params (DeltaSeconds :type "Float (single-precision)")))

(event `self.Sphere.OnInputTouchBegin`
  (params (FingerIndex :type "ETouchIndex Enum" :default "Touch1") (TouchedComponent :type "PrimitiveComponent Object Reference"))
  (`self.ZoomLocation` (`self.LocationNumber`)))

(event `self.ZoneMesh.OnInputTouchBegin`
  (params (FingerIndex :type "ETouchIndex Enum" :default "Touch1") (TouchedComponent :type "PrimitiveComponent Object Reference"))
  (`self.CheckPositionAndZoom` (`self.LocationNumber`)))

(fn `CheckPositionAndZoom`
  (params (LocationNumber :type Integer))
  (bind _returnvalue_x (`KismetMathLibrary.BreakVector` (`self.K2_GetActorLocation` (`GameplayStatics.GetPlayerPawn` 0))))
  (bind _asbp_main_game_instance (`/Game/TopDown/Blueprints/CommonFunctionsLibrary.GetGameInstance`))
  (if (< _returnvalue_x 124.0)
    (`self.ZoomLocation` LocationNumber)
    (if (== (`/Game/LevelsParameters/Storing/StoringPawn.FoodRef` (`self.PawnRef`)) null)
      (`|ExecutionSequence`
        (:`then_0`
          (bind _foundwidgets (`WidgetBlueprintLibrary.GetAllWidgetsOfClass` "/Game/UIElements/WBP_CommonUI.WBP_CommonUI_C"))
          (bind _language (`/Game/TopDown/Blueprints/BP_MainGameInstance.Language` _asbp_main_game_instance))
          (switch `string` _language
            (:`pt`
              (bind _output (`|GetArrayItem` _foundwidgets))
              (set `/Game/UIElements/WBP_CommonUI.DialogueString` "Antes de entrares na zona de arrumação seleciona a comida do cesto, para voltares atrás tens o círculo à esquerda." _output))
            (:`en`
              (set `/Game/UIElements/WBP_CommonUI.DialogueString` "Select the food from the basket before joinning a storing zone, go back by pressing on the circule in the left." _output)))
          (`Widget.SetVisibility` (`/Game/UIElements/WBP_CommonUI.DialogueContainer` _output) "Visible")
          (`Widget.SetVisibility` (`/Game/UIElements/WBP_CommonUI.BackButton` _output) "Visible")
          (`/Game/UIElements/WBP_CommonUI.SetImage` _output "Back")
          (`Widget.SetVisibility` (`/Game/UIElements/WBP_CommonUI.ChefimgButton` _output) "Hidden")
          (`Widget.SetVisibility` (`/Game/UIElements/WBP_CommonUI.ChefOlivia` _output) "Hidden")))
      (else
        (`|ExecutionSequence`
          (:`then_1`
            (if (`self.C1`)
              (bind _foundwidgets_2 (`WidgetBlueprintLibrary.GetAllWidgetsOfClass` "/Game/UIElements/WBP_CommonUI.WBP_CommonUI_C"))
              (switch `string` _language
                (:`pt`
                  (set `/Game/UIElements/WBP_CommonUI.DialogueString` "Tem atenção à comida e às prateleiras faz um swipe quando quiseres arrumá-la, para voltar atrás tens o círculo à esquerda." (`|GetArrayItem` _foundwidgets_2)))
                (:`en`
                  (bind _output_2 (`|GetArrayItem` (stale _foundwidgets_4)))
                  (set `/Game/UIElements/WBP_CommonUI.DialogueString` "Pay attention to the food and the shelves, perform a swipe when you want to store it, go back by pressing in the circule at the left." _output_2)))
              (`self.ShowBackButton` :!label _label)
              (else
                (bind _foundwidgets_3 (`WidgetBlueprintLibrary.GetAllWidgetsOfClass` "/Game/UIElements/WBP_CommonUI.WBP_CommonUI_C"))
                (switch `string` _language
                  (:`pt`
                    (bind _output_3 (`|GetArrayItem` _foundwidgets_3))
                    (set `/Game/UIElements/WBP_CommonUI.DialogueString` "Tem atenção à comida e às prateleiras faz um swipe quando quiseres arrumá-la, para voltar atrás tens o círculo à esquerda." _output_3))
                  (:`en`
                    (set `/Game/UIElements/WBP_CommonUI.DialogueString` "Pay attention to the food and the shelves, perform a swipe when you want to store it, go back by pressing in the circule at the left." _output_3)))
                (`Widget.SetVisibility` (`/Game/UIElements/WBP_CommonUI.DialogueContainer` _output_3) "Visible")
                (`Widget.SetVisibility` (`/Game/UIElements/WBP_CommonUI.BackButton` _output_3) "Visible")
                (`/Game/UIElements/WBP_CommonUI.SetImage` _output_3 "Back")
                (`Widget.SetVisibility` (`/Game/UIElements/WBP_CommonUI.ChefimgButton` _output_3) "Hidden")
                (`Widget.SetVisibility` (`/Game/UIElements/WBP_CommonUI.ChefOlivia` _output_3) "Hidden")
                (set `self.C1` true)
                (bind _outactors (`GameplayStatics.GetAllActorsOfClass` "BP_SelectArea_C"))
                (for _array_element _outactors
                  (set `/Game/LevelsParameters/Storing/BP_SelectArea.C1` true _array_element))))))))
    (else
      (`|ExecutionSequence`
        (:`then_1`
          (if (`self.C2`)
            (bind _foundwidgets_4 (`WidgetBlueprintLibrary.GetAllWidgetsOfClass` "/Game/UIElements/WBP_CommonUI.WBP_CommonUI_C"))
            (switch `string` _language
              (:`pt`
                (set `/Game/UIElements/WBP_CommonUI.DialogueString` "Volta atrás clicando no círculo à esquerda com a seta, para arrumares a comida faz um swipe no ecrã, tem atenção à posição da seta." _output_2)
                (goto _label))
              (:`en`
                (set `/Game/UIElements/WBP_CommonUI.DialogueString` "Go back by pressing in the circle with an arrow at the left, to store perform a swipe in the screen, pay attention to the arrow's position." _output_2)
                (goto _label)))
            (else
              (bind _foundwidgets_5 (`WidgetBlueprintLibrary.GetAllWidgetsOfClass` "/Game/UIElements/WBP_CommonUI.WBP_CommonUI_C"))
              (switch `string` _language
                (:`pt`
                  (bind _output_4 (`|GetArrayItem` _foundwidgets_5))
                  (set `/Game/UIElements/WBP_CommonUI.DialogueString` "Volta atrás clicando no círculo à esquerda com a seta, para arrumares a comida faz um swipe no ecrã, tem atenção à posição da seta." _output_4))
                (:`en`
                  (set `/Game/UIElements/WBP_CommonUI.DialogueString` "Go back by pressing in the circle with an arrow at the left, to store perform a swipe in the screen, pay attention to the arrow's position." _output_4)))
              (`Widget.SetVisibility` (`/Game/UIElements/WBP_CommonUI.DialogueContainer` _output_4) "Visible")
              (`Widget.SetVisibility` (`/Game/UIElements/WBP_CommonUI.BackButton` _output_4) "Visible")
              (`/Game/UIElements/WBP_CommonUI.SetImage` _output_4 "Back")
              (`Widget.SetVisibility` (`/Game/UIElements/WBP_CommonUI.ChefimgButton` _output_4) "Hidden")
              (`Widget.SetVisibility` (`/Game/UIElements/WBP_CommonUI.ChefOlivia` _output_4) "Hidden")
              (set `self.C2` true)
              (bind _outactors_2 (`GameplayStatics.GetAllActorsOfClass` "BP_SelectArea_C"))
              (for _array_element_2 _outactors_2
                (set `/Game/LevelsParameters/Storing/BP_SelectArea.C2` true _array_element_2)))))))))

(fn `SetVisibleZoneFood`
  (params (FilledZoneName :type String) (CZone :type Boolean))
  (if (== (`/Game/LevelsParameters/Storing/Structures/Storing_Manager.CurrentDay` (`/Game/LevelsParameters/Storing/StoringPawn.StoringManager` (`self.PawnRef`))) "Day1")
    (if (not CZone)
      (bind _outactors (`GameplayStatics.GetAllActorsOfClass` "/Script/Engine.StaticMeshActor"))
      (for _array_element _outactors
        (if (== (`KismetSystemLibrary.GetDisplayName` _array_element) FilledZoneName)
          (`SceneComponent.SetVisibility` (`StaticMeshActor.StaticMeshComponent` _array_element) true true)))
      (bind _foundwidgets (`WidgetBlueprintLibrary.GetAllWidgetsOfClass` "/Game/UIElements/WBP_CommonUI.WBP_CommonUI_C"))
      (bind _asbp_main_game_instance (`/Game/TopDown/Blueprints/CommonFunctionsLibrary.GetGameInstance`))
      (switch `string` (`/Game/TopDown/Blueprints/BP_MainGameInstance.Language` _asbp_main_game_instance)
        (:`pt`
          (bind _dialoguestringtemp (`/Game/UIElements/WBP_CommonUI.DialogueStringTemp` (`|GetArrayItem` _foundwidgets)))
          (`KismetArrayLibrary.Array_Add` _dialoguestringtemp "Como podes observar estes são os alimentos que podes arrumar nesta zona, em cada prateleira em específico."))
        (:`en`
          (`KismetArrayLibrary.Array_Add` _dialoguestringtemp "As you can see this is the food that you can store in this area, in each shelf specifically.")))
      (return))))

(fn `ShowBackButton`
  (bind _foundwidgets (`WidgetBlueprintLibrary.GetAllWidgetsOfClass` "/Game/UIElements/WBP_CommonUI.WBP_CommonUI_C"))
  (bind _output (`|GetArrayItem` _foundwidgets))
  (`Widget.SetVisibility` (`/Game/UIElements/WBP_CommonUI.BackButton` _output) "Visible")
  (`Widget.SetVisibility` (`/Game/UIElements/WBP_CommonUI.ShowTextHighlight` _output) "Visible")
  (`/Game/UIElements/WBP_CommonUI.BlinkIcon` _output))

(fn `StartPositiioin`
  (params (SelfComponent :type "SceneComponent Object Reference"))
  (`SceneComponent.K2_SetRelativeLocation` SelfComponent (123.508975 -13.768993 200.0) false false)
  (bind _outactors (`GameplayStatics.GetAllActorsOfClass` "/Game/LevelsParameters/Storing/BP_StoringArrow.BP_StoringArrow_C"))
  (`self.K2_DestroyActor` _outactors)
  (bind _outactors_2 (`GameplayStatics.GetAllActorsOfClass` "/Script/Engine.TextRenderActor"))
  (for _array_element _outactors_2
    (bind _textrender (`TextRenderActor.TextRender` _array_element))
    (if (`KismetStringLibrary.Contains` (`KismetSystemLibrary.GetDisplayName` _textrender) "shelf" false true)
      (`SceneComponent.SetVisibility` _textrender false true)
      (elif (`KismetStringLibrary.Contains` (`KismetSystemLibrary.GetDisplayName` _array_element) "zone" false true)
        (`SceneComponent.SetVisibility` (`TextRenderActor.TextRender` _array_element) true true))))
  (bind _foundwidgets (`WidgetBlueprintLibrary.GetAllWidgetsOfClass` "/Game/UIElements/WBP_CommonUI.WBP_CommonUI_C"))
  (`Widget.SetVisibility` (`/Game/UIElements/WBP_CommonUI.BackButton` (`|GetArrayItem` _foundwidgets)) "Hidden")
  (bind _outactors_3 (`GameplayStatics.GetAllActorsOfClass` "BP_SelectArea_C"))
  (for _array_element_2 _outactors_3
    (if (== (`/Game/LevelsParameters/Storing/BP_SelectArea.LocationNumber` _array_element_2) 546)
      (`SceneComponent.SetVisibility` (`/Game/LevelsParameters/Storing/BP_SelectArea.ZoneMesh` _array_element_2) false true)))
  (bind _foundwidgets_2 (`WidgetBlueprintLibrary.GetAllWidgetsOfClass` "/Game/UIElements/WBP_SwipeClue.WBP_SwipeClue_C"))
  (for _array_element_3 _foundwidgets_2
    (`Widget.RemoveFromParent` _array_element_3))
  (bind _outactors_4 (`GameplayStatics.GetAllActorsOfClass` "/Script/Engine.StaticMeshActor"))
  (for _array_element_4 _outactors_4
    (if (`KismetStringLibrary.Contains` (`KismetSystemLibrary.GetDisplayName` _array_element_4) "Filled")
      (`SceneComponent.SetVisibility` (`StaticMeshActor.StaticMeshComponent` _array_element_4) false true))))

(fn `UserConstructionScript`
  (`MeshComponent.SetOverlayMaterial` (`self.ZoneMesh`) (`self.Material`)))

(fn `ZoomLocation`
  (params (LocationNumber :type Integer))
  (bind _locationnumber (`self.LocationNumber`))
  (bind _defaultsceneroot (`/Game/LevelsParameters/Storing/StoringPawn.DefaultSceneRoot` (`self.PawnRef`)))
  (switch `int` LocationNumber
    (:`Default`
      ;[1 1 1] Start position
      (`self.StartPositiioin` _defaultsceneroot)
      (bind _outactors (`GameplayStatics.GetAllActorsOfClass` "BP_SelectArea_C"))
      (for _array_element _outactors
        (set `/Game/LevelsParameters/Storing/BP_SelectArea.Material` (`/Game/LevelsParameters/Storing/BP_SelectArea.MaterialRef` _array_element) _array_element)
        (`MeshComponent.SetOverlayMaterial` (`/Game/LevelsParameters/Storing/BP_SelectArea.ZoneMesh` _array_element) (`/Game/LevelsParameters/Storing/BP_SelectArea.Material` _array_element)))
      (`SceneComponent.SetVisibility` (`/Game/LevelsParameters/Storing/StoringPawn.Arrow` (`self.PawnRef`)) false false))
    (:`1`
      (`|ExecutionSequence`
        (:`then_0`
          (`self.SetVisibleZoneFood` "PantryFilled" (`self.CPantry`))
          (set `self.CPantry` true))
        (:`then_1`
          ;[1 1 1] Pantry
          (`SceneComponent.K2_SetRelativeLocation` _defaultsceneroot (588.713169 -550.673519 200.0) false false)
          (bind _outactors_2 (`GameplayStatics.GetAllActorsOfClass` "/Game/LevelsParameters/Storing/BP_StoringArrow.BP_StoringArrow_C"))
          (if (`KismetArrayLibrary.Array_IsEmpty` _outactors_2)
            ;[1 1 1] Rever valores StoringLocations
            (`|SpawnActorFromClass` "/Game/LevelsParameters/Storing/BP_StoringArrow.BP_StoringArrow_C" (`KismetMathLibrary.MakeTransform` (972.506804 -320.589387 20.72)) "Undefined" "OverrideRootScale" null _locationnumber 280.0 20.0 1.0 null)
            (bind _outactors_3 (`GameplayStatics.GetAllActorsOfClass` "/Script/Engine.TextRenderActor" :!label _label))
            (for _array_element_2 _outactors_3
              (if (`KismetStringLibrary.Contains` (`KismetSystemLibrary.GetDisplayName` _array_element_2) "shelf" false true)
                (`SceneComponent.SetVisibility` (`TextRenderActor.TextRender` _array_element_2) true true)
                (elif (`KismetStringLibrary.Contains` (`KismetSystemLibrary.GetDisplayName` _array_element_2) "zone" false true)
                  (`SceneComponent.SetVisibility` (`TextRenderActor.TextRender` _array_element_2) false true))))
            (bind _outactors_4 (`GameplayStatics.GetAllActorsOfClass` "BP_SelectArea_C"))
            (for _array_element_3 _outactors_4
              (if (not (== _array_element_3 self))
                (`MeshComponent.SetOverlayMaterial` (`/Game/LevelsParameters/Storing/BP_SelectArea.ZoneMesh` _array_element_3) null)))
            (`SceneComponent.SetVisibility` (`/Game/LevelsParameters/Storing/StoringPawn.Arrow` (`self.PawnRef`)) true false)
            (if (not (== (`/Game/LevelsParameters/Storing/StoringPawn.FoodRef` (`self.PawnRef`)) null))
              (bind _asstoring_pawn (`/Game/TopDown/Blueprints/CommonFunctionsLibrary.GetStoringPawn`))
              (if (== (`/Game/LevelsParameters/Storing/Structures/Storing_Manager.CurrentDay` (`/Game/LevelsParameters/Storing/StoringPawn.StoringManager` _asstoring_pawn)) "Day1")
                (bind _returnvalue (`|CreateWidget` "/Game/UIElements/WBP_SwipeClue.WBP_SwipeClue_C"))
                (`UserWidget.AddToViewport` _returnvalue 0)))))))
    (:`2`
      (`|ExecutionSequence`
        (:`then_0`
          (`self.SetVisibleZoneFood` "FilledFridge" (`self.CFridge`))
          (set `self.CFridge` true))
        (:`then_1`
          ;[1 1 1] Fridge
          (`SceneComponent.K2_SetRelativeLocation` _defaultsceneroot (588.713169 -4.613227 440.0) false false)
          (bind _outactors_5 (`GameplayStatics.GetAllActorsOfClass` "/Game/LevelsParameters/Storing/BP_StoringArrow.BP_StoringArrow_C"))
          (if (not (`KismetArrayLibrary.Array_IsEmpty` _outactors_5))
            (`self.K2_DestroyActor` _outactors_5))
          (`|SpawnActorFromClass` "/Game/LevelsParameters/Storing/BP_StoringArrow.BP_StoringArrow_C" (`KismetMathLibrary.MakeTransform` (972.506804 203.0 230.72)) "Undefined" "OverrideRootScale" null _locationnumber 524.0 230.0 1.0 null)
          (goto _label))))
    (:`3`
      (`|ExecutionSequence`
        (:`then_0`
          (`self.SetVisibleZoneFood` "FilledFreezer" (`self.CFreezer`))
          (set `self.CFreezer` true))
        (:`then_1`
          ;[1 1 1] Freezer
          (`SceneComponent.K2_SetRelativeLocation` _defaultsceneroot (588.713169 -4.613227 200.0) false false)
          (bind _outactors_6 (`GameplayStatics.GetAllActorsOfClass` "/Game/LevelsParameters/Storing/BP_StoringArrow.BP_StoringArrow_C"))
          (if (not (`KismetArrayLibrary.Array_IsEmpty` _outactors_6))
            (`self.K2_DestroyActor` _outactors_6))
          (`|SpawnActorFromClass` "/Game/LevelsParameters/Storing/BP_StoringArrow.BP_StoringArrow_C" (`KismetMathLibrary.MakeTransform` (972.506804 203.0 20.72)) "Undefined" "OverrideRootScale" null _locationnumber 203.0 20.0 1.0 null)
          (goto _label))))))