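; Touchable customization option actor that equips its row and category on the player's BP_TopDownCharacter when unlocked.
; A successful touch plays one of two wearing sounds, depending on whether the row name contains "Empty".
; A locked touch shows a timed English or Portuguese warning through WBP_CommonUI.
; Helper functions display the required level via widget and text render, and set or clear a locked overlay material.
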(event `self.StaticMesh.OnInputTouchBegin`
  (params (FingerIndex :type "ETouchIndex Enum" :default "Touch1") (TouchedComponent :type "PrimitiveComponent Object Reference"))
  (bind _returnvalue (`self.K2_GetActorLocation` (`GameplayStatics.GetPlayerPawn` 0)))
  (if (`self.isUnlocked`)
    (`self.ChangeMesh`)
    (if (`KismetStringLibrary.Contains` (`KismetStringLibrary.Conv_NameToString` (`self.RowName`)) "Empty")
      (`GameplayStatics.PlaySoundAtLocation` "/Game/LevelsParameters/Customization/SFX/WearingClothesSFX.WearingClothesSFX" _returnvalue (struct) 1.0 1.0 0.0 null null null null)
      (else
        (`GameplayStatics.PlaySoundAtLocation` "/Game/LevelsParameters/Customization/SFX/WearingClothesSFX2.WearingClothesSFX2" _returnvalue (struct) 1.0 1.0 0.0 null null null null)))
    (else
      (bind _foundwidgets (`WidgetBlueprintLibrary.GetAllWidgetsOfClass` "/Game/UIElements/WBP_CommonUI.WBP_CommonUI_C"))
      (bind _asbp_main_game_instance (`/Game/TopDown/Blueprints/CommonFunctionsLibrary.GetGameInstance`))
      (switch `string` (`/Game/TopDown/Blueprints/BP_MainGameInstance.Language` _asbp_main_game_instance)
        (:`en`
          (bind _output (`|GetArrayItem` _foundwidgets))
          (set `/Game/UIElements/WBP_CommonUI.DialogueString` "You have not unlocked that option." _output))
        (:`pt`
          (set `/Game/UIElements/WBP_CommonUI.DialogueString` "Ainda não desbloqueaste essa opção." _output)))
      (`Widget.SetVisibility` (`/Game/UIElements/WBP_CommonUI.DialogueContainer` _output) "Visible")
      (`/Game/UIElements/WBP_CommonUI.CheckTime` _output 1.3))))

(fn `ChangeMesh`
  (bind _output_get (set `self.Character` (`GameplayStatics.GetPlayerCharacter` 0)))
  (bind _asbp_top_down_character (cast `/Game/TopDown/Blueprints/BP_TopDownCharacter` _output_get))
  (`/Game/TopDown/Blueprints/BP_TopDownCharacter.EquipCustomization` _asbp_top_down_character (`self.RowName`) (`self.Category`)))

(fn `SetDisableMaterial`
  (`MeshComponent.SetOverlayMaterial` (`self.StaticMesh`) "/Game/LevelsParameters/Customization/MeshesAndMaterials/MI_NotUnlocked.MI_NotUnlocked"))

(fn `SetEnableMaterial`
  (`MeshComponent.SetOverlayMaterial` (`self.StaticMesh`) null))

(fn `SetLevelRequired`
  (params (LevelReq :type "Integer (by ref)"))
  (bind _textrender (`self.TextRender`))
  (bind _returnvalue (`|CreateWidget` "/Game/UIElements/WBP_LevelRequired.WBP_LevelRequired_C" null LevelReq (`self.isUnlocked`)))
  (`WidgetComponent.SetWidget` (`self.LevelRequiredImg`) _returnvalue)
  (`TextRenderComponent.K2_SetText` _textrender (`KismetTextLibrary.Conv_IntToText` LevelReq))
  (`SceneComponent.SetHiddenInGame` _textrender false false))

(fn `UserConstructionScript`)