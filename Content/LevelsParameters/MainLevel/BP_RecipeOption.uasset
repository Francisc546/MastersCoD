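; BP_RecipeOption is a touchable food choice in the main level that starts a recipe.
; Its mesh comes from the game instance's food data at GameInstanceIndex.
; Selection reports the pick to MainHUB_Manager, shows the first instruction in the common UI, removes that food from the stored arrays and sets the active recipe.
; It then reveals and moves the slicing level-change zone and destroys every recipe option.
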(event `self.ReceiveBeginPlay`
  (bind _cube (`self.Cube`))
  (if (== (`KismetSystemLibrary.GetDisplayName` (`StaticMeshComponent.StaticMesh` _cube)) "Butter")
    (`PrimitiveComponent.SetMaterial` _cube 0 "/Game/LevelsParameters/MeshesAndMaterials/MaterialsTextures/YellowGoodButter.YellowGoodButter")))

(event `self.ReceiveTick`
  (params (DeltaSeconds :type "Float (single-precision)")))

(event `SelectFood`
  (bind _output (`|GetArrayItem` (`/Game/LevelsParameters/Cooking/Structures/RecipeDataAsset.RecipeInstructions` (`self.Recipe`))))
  (bind _outactors (`GameplayStatics.GetAllActorsOfClass` "/Game/LevelsParameters/MainLevel/MainHUB_Manager.MainHUB_Manager_C" :!label _label))
  (`GameplayStatics.PlaySound2D` "/Game/LevelsParameters/InteractFood2.InteractFood2" 1.0 1.0 0.0 null null)
  (`/Game/LevelsParameters/MainLevel/MainHUB_Manager.AddRecipeEvaluation` (`|GetArrayItem` _outactors) (`self.GameInstanceIndex`))
  (bind _foundwidgets (`WidgetBlueprintLibrary.GetAllWidgetsOfClass` "/Game/UIElements/WBP_CommonUI.WBP_CommonUI_C"))
  (bind _output_2 (`|GetArrayItem` _foundwidgets))
  (`Widget.SetVisibility` (`/Game/UIElements/WBP_CommonUI.DialogueContainer` _output_2) "Visible")
  (set `/Game/UIElements/WBP_CommonUI.DialogueString` (`KismetTextLibrary.Conv_TextToString` _output) _output_2)
  (set `/Game/UIElements/WBP_CommonUI.RecipeString` (`KismetTextLibrary.Conv_TextToString` _output) _output_2)
  (bind _foundwidgets_2 (`WidgetBlueprintLibrary.GetAllWidgetsOfClass` "/Game/UIElements/WBP_Recipe.WBP_Recipe_C"))
  (`Widget.RemoveFromParent` (`|GetArrayItem` _foundwidgets_2))
  (bind _asbp_main_game_instance (`self.RemoveFoodGameInstance`))
  (set `/Game/TopDown/Blueprints/BP_MainGameInstance.ActiveRecipe` (`self.Recipe`) _asbp_main_game_instance)
  (`self.EnableSlicingLevel`)
  (bind _outactors_2 (`GameplayStatics.GetAllActorsOfClass` "BP_RecipeOption_C"))
  (for _array_element _outactors_2
    (`self.K2_DestroyActor` _array_element)))

(event `self.Cube.OnInputTouchBegin`
  (params (FingerIndex :type "ETouchIndex Enum" :default "Touch1") (TouchedComponent :type "PrimitiveComponent Object Reference"))
  (goto _label))

(fn `EnableSlicingLevel`
  (bind _outactors (`GameplayStatics.GetAllActorsOfClass` "/Game/TopDown/Blueprints/BP_ChangeLevelZone.BP_ChangeLevelZone_C"))
  (for _array_element _outactors
    (if (== (`KismetSystemLibrary.GetDisplayName` _array_element) "BP_ChangeLevelSlicing")
      (`self.SetActorHiddenInGame` _array_element false)
      (`SceneComponent.K2_SetWorldLocation` (`/Game/TopDown/Blueprints/BP_ChangeLevelZone.DefaultSceneRoot` _array_element) (587.667041 3515.988017 53.8237) false false)
      ;[1 1 1] Little fix to not show up on screen o.O
      (bind _foundwidgets (`WidgetBlueprintLibrary.GetAllWidgetsOfClass` "/Game/UIElements/WBP_ChangeLevel.WBP_ChangeLevel_C"))
      (for _array_element_2 _foundwidgets
        (`Widget.RemoveFromParent` _array_element_2))))
  (return))

(fn `RemoveFoodGameInstance`
  (returns (`AsBP Main Game Instance` :type "/Game/TopDown/Blueprints/BP_MainGameInstance Object Reference"))
  (bind _gameinstanceindex (`self.GameInstanceIndex`))
  (bind _asbp_main_game_instance (cast `/Game/TopDown/Blueprints/BP_MainGameInstance` (`GameplayStatics.GetGameInstance`)))
  (`KismetArrayLibrary.Array_Remove` (`/Game/TopDown/Blueprints/BP_MainGameInstance.FoodDataElement` _asbp_main_game_instance) _gameinstanceindex)
  (`KismetArrayLibrary.Array_Remove` (`/Game/TopDown/Blueprints/BP_MainGameInstance.FoodExpiryElement` _asbp_main_game_instance) _gameinstanceindex)
  (`KismetArrayLibrary.Array_Remove` (`/Game/TopDown/Blueprints/BP_MainGameInstance.StoredZoneString` _asbp_main_game_instance) _gameinstanceindex)
  (return _asbp_main_game_instance))

(fn `UserConstructionScript`
  (bind _asbp_main_game_instance (cast `/Game/TopDown/Blueprints/BP_MainGameInstance` (`GameplayStatics.GetGameInstance`)))
  (`StaticMeshComponent.SetStaticMesh` (`self.Cube`) (`/Game/LevelsParameters/Storing/Structures/FoodDataAsset.Mesh` (`|GetArrayItem` (`/Game/TopDown/Blueprints/BP_MainGameInstance.FoodDataElement` _asbp_main_game_instance) (`self.GameInstanceIndex`)))))