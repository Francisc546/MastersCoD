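; Cleaning plate actor that scatters leftover bad food on itself and turns on the sink water when play begins.
; SpawnBadFoodPieces drains the game instance's BadFoodOutsideRecipe counter, spawning one apple-quarter BP_BadFood with the bad-food material per count at a random offset just above the plate.
; BeginPlay then searches all static mesh actors and makes those tagged SinkWater visible.
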(event `self.ReceiveBeginPlay`
  (`self.SpawnBadFoodPieces`)
  (bind _outactors (`GameplayStatics.GetAllActorsOfClass` "/Script/Engine.StaticMeshActor"))
  (for _array_element _outactors
    (for _array_element_2 (`Actor.Tags` _array_element)
      (if (== _array_element_2 "SinkWater")
        (`SceneComponent.SetVisibility` (`StaticMeshActor.StaticMeshComponent` _array_element) true false)))))

(event `self.ReceiveTick`
  (params (DeltaSeconds :type "Float (single-precision)")))

(fn `SpawnBadFoodPieces`
  (bind _returnvalue (`self.GetTransform` self))
  (bind _asbp_main_game_instance (`/Game/TopDown/Blueprints/CommonFunctionsLibrary.GetGameInstance`))
  (bind _badfoodoutsiderecipe (`/Game/TopDown/Blueprints/BP_MainGameInstance.BadFoodOutsideRecipe` _asbp_main_game_instance))
  (while (>= _badfoodoutsiderecipe 1)
    (bind _returnvalue_2 (`|SpawnActorFromClass` "/Game/LevelsParameters/MainLevel/BP_BadFood.BP_BadFood_C" (`KismetMathLibrary.MakeTransform` (`KismetMathLibrary.MakeVector` (+ (`KismetMathLibrary.RandomFloatInRange` -40.0 40.0) (.x (.location _returnvalue))) (+ (`KismetMathLibrary.RandomFloatInRange` -40.0 40.0) (.y (.location _returnvalue))) (+ (.z (.location _returnvalue)) 2.0)) (struct) (0.6 0.6 0.6)) "Undefined" "OverrideRootScale" null "/Game/LevelsParameters/MeshesAndMaterials/Slices/Apple_Quarter.Apple_Quarter" null))
    (`PrimitiveComponent.SetMaterial` (`/Game/LevelsParameters/MainLevel/BP_BadFood.Cube` _returnvalue_2) 0 "/Game/LevelsParameters/SlicingTesting/UnrealExample/M_BadFood.M_BadFood")
    (`/Engine/EditorBlueprintResources/StandardMacros.DecrementInt` _badfoodoutsiderecipe))
  (return))

(fn `UserConstructionScript`)