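; BP_RecipeBook is the tappable recipe book in the main level that starts recipe selection based on food closest to expiring.
; Entering its box shows Chef Olivia's dialogue in English or Portuguese, gated by a DoOnce that resets on exit.
; Touching the book, if no recipe widget exists, spawns two BP_RecipeOption actors from hub manager and GameInstance data.
; It then updates the dialogue, has MainHUB_Manager spawn the recipes widget, and removes itself.
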(event `self.ReceiveBeginPlay`
  (bind _outactors (`GameplayStatics.GetAllActorsOfClass` "/Game/LevelsParameters/MainLevel/MainHUB_Manager.MainHUB_Manager_C"))
  (set `self.MainHUBManagerRef` (`|GetArrayItem` _outactors)))

(event `self.ReceiveTick`
  (params (DeltaSeconds :type "Float (single-precision)")))

(event `self.Box.OnComponentBeginOverlap`
  (params (OverlappedComponent :type "PrimitiveComponent Object Reference") (OtherActor :type "Actor Object Reference") (OtherComp :type "PrimitiveComponent Object Reference") (OtherBodyIndex :type Integer) (bFromSweep :type Boolean) (SweepResult :type "HitResult Structure (by ref)"))
  (`/Engine/EditorBlueprintResources/StandardMacros.DoOnce` false :!label _label
    (:`Completed`
      (bind _foundwidgets (`WidgetBlueprintLibrary.GetAllWidgetsOfClass` "/Game/UIElements/WBP_CommonUI.WBP_CommonUI_C"))
      (bind _output (`|GetArrayItem` _foundwidgets))
      (`Widget.SetVisibility` (`/Game/UIElements/WBP_CommonUI.DialogueContainer` _output) "Visible")
      (`Widget.SetVisibility` (`/Game/UIElements/WBP_CommonUI.ChefOlivia` _output) "Visible")
      (`Widget.SetVisibility` (`/Game/UIElements/WBP_CommonUI.ChefimgButton` _output) "Visible")
      (bind _asbp_main_game_instance (`/Game/TopDown/Blueprints/CommonFunctionsLibrary.GetGameInstance`))
      (switch `string` (`/Game/TopDown/Blueprints/BP_MainGameInstance.Language` _asbp_main_game_instance)
        (:`en`
          (set `/Game/UIElements/WBP_CommonUI.DialogueString` "Press in the book that's on the table to select a recipe, choose the recipe with the food that has the expiry period closer to expirying." _output))
        (:`pt`
          (set `/Game/UIElements/WBP_CommonUI.DialogueString` "Clica no livro da mesa para escolheres a receita, escolhe a receita com o alimento que tem o prazo de validade mais próximo de expirar." _output))))))

(event `self.Box.OnComponentEndOverlap`
  (params (OverlappedComponent :type "PrimitiveComponent Object Reference") (OtherActor :type "Actor Object Reference") (OtherComp :type "PrimitiveComponent Object Reference") (OtherBodyIndex :type Integer))
  (goto _label :!via `Reset`))

(event `self.Cube.OnClicked`
  (params (TouchedComponent :type "PrimitiveComponent Object Reference") (ButtonPressed :type "Key Structure")))

(event `self.Cube.OnInputTouchBegin`
  (params (FingerIndex :type "ETouchIndex Enum" :default "Touch1") (TouchedComponent :type "PrimitiveComponent Object Reference"))
  (bind _foundwidgets (`WidgetBlueprintLibrary.GetAllWidgetsOfClass` "/Game/UIElements/WBP_Recipe.WBP_Recipe_C"))
  (if (== (`KismetArrayLibrary.Array_Length` _foundwidgets) 0)
    ;[1 1 1] Display Recipe options Widget
    (`self.SpawnRecipeOptions`)
    (bind _asbp_main_game_instance (`/Game/TopDown/Blueprints/CommonFunctionsLibrary.GetGameInstance`))
    (switch `string` (`/Game/TopDown/Blueprints/BP_MainGameInstance.Language` _asbp_main_game_instance)
      (:`en`
        (bind _output (`|GetArrayItem` (stale `self.Box.OnComponentBeginOverlap` _foundwidgets)))
        (set `/Game/UIElements/WBP_CommonUI.DialogueString` "Press on the food that's on the table to select the recipe to cook." _output)
        (`KismetArrayLibrary.Array_Add` (`/Game/UIElements/WBP_CommonUI.DialogueStringTemp` _output) "Remember to select the food that's closer to expirying for the recipe."))
      (:`pt`
        (set `/Game/UIElements/WBP_CommonUI.DialogueString` "Clica na comida que está na mesa para selecionares a receita para cozinhares." _output)
        (`KismetArrayLibrary.Array_Add` (`/Game/UIElements/WBP_CommonUI.DialogueStringTemp` _output) "Lembra-te de escolher a comida com o número menor de dias para a nossa receita.")))
    (`/Game/LevelsParameters/MainLevel/MainHUB_Manager.SpawnRecipesWidget` (`self.MainHUBManagerRef`))
    (`self.SetLifeSpan` 0.01)))

(fn `SpawnRecipeOptions`
  (bind _recipearray (`/Game/LevelsParameters/MainLevel/MainHUB_Manager.RecipeArray` (`self.MainHUBManagerRef`)))
  (bind _asbp_main_game_instance (`/Game/TopDown/Blueprints/CommonFunctionsLibrary.GetGameInstance`))
  (bind _fooddataelement (`/Game/TopDown/Blueprints/BP_MainGameInstance.FoodDataElement` _asbp_main_game_instance))
  (`|SpawnActorFromClass` "/Game/LevelsParameters/MainLevel/BP_RecipeOption.BP_RecipeOption_C" (`KismetMathLibrary.MakeTransform` (773.628177 497.69179 79.080471) (struct) (0.5 0.5 0.5)) "Undefined" "OverrideRootScale" null (`|GetArrayItem` _recipearray) 0 (`/Game/LevelsParameters/Storing/Structures/FoodDataAsset.Name` (`|GetArrayItem` _fooddataelement)) null)
  (`|SpawnActorFromClass` "/Game/LevelsParameters/MainLevel/BP_RecipeOption.BP_RecipeOption_C" (`KismetMathLibrary.MakeTransform` (773.628177 655.26874 79.080471) (struct) (0.5 0.5 0.5)) "Undefined" "OverrideRootScale" null (`|GetArrayItem` _recipearray 1) 1 (`/Game/LevelsParameters/Storing/Structures/FoodDataAsset.Name` (`|GetArrayItem` _fooddataelement 1)) null))

(fn `UserConstructionScript`)