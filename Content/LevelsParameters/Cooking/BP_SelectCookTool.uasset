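; Touch-selectable pot, pan or plate for the cooking level, with its tool type derived from the mesh name.
; A touch moves the tool to the cook position, destroys the others and notifies the pawn's CookingManager.
; Pot and pan advance through a water-fill step with Tick-scaled water, steam and boiling sound, while plate skips it.
; Both paths then switch to the cutting table, spawn slicing food and update recipe and dialogue text.
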(event `self.ReceiveTick`
  (params (DeltaSeconds :type "Float (single-precision)"))
  (bind _water (`self.Water`))
  (bind (_returnvalue_x _returnvalue_y) (`KismetMathLibrary.BreakVector` (`SceneComponent.K2_GetComponentScale` _water)))
  (`SceneComponent.SetWorldScale3D` _water (`KismetMathLibrary.MakeVector` _returnvalue_x _returnvalue_y (`self.WaterHeight`))))

(event `self.ReceiveBeginPlay`
  (`self.SetToolType`)
  (`/Engine/EditorBlueprintResources/StandardMacros.IsValid` (`self.PawnRef`)
    (:`Is Not Valid`
      (bind _asslice_game_pawn (`/Game/TopDown/Blueprints/CommonFunctionsLibrary.GetSlicingPawn`))
      (set `self.PawnRef` _asslice_game_pawn)
      (if (== (`KismetSystemLibrary.GetObjectName` (`self.ToolMesh`)) "Pan")
        (`SceneComponent.K2_SetRelativeLocation` (`self.Water`) (0.0 -15.0 0.0) false false)))))

(event `self.StaticMesh.OnInputTouchBegin`
  (params (FingerIndex :type "ETouchIndex Enum" :default "Touch1") (TouchedComponent :type "PrimitiveComponent Object Reference"))
  (bind _pawnref (`self.PawnRef`))
  (bind _tooltype (`self.ToolType`))
  (bind _pawnref_2 (`self.PawnRef`))
  (bind _slicingmanager (`/Game/LevelsParameters/SlicingTesting/UnrealExample/SliceGamePawn.SlicingManager` _pawnref))
  (bind _currentstep (`/Game/LevelsParameters/SlicingTesting/UnrealExample/SliceGamePawn.CurrentStep` _pawnref_2))
  (bind _returnvalue (> _currentstep 1))
  (bind _slicingfoodcount (`/Game/LevelsParameters/SlicingTesting/Structures/Slicing_Manager.SlicingFoodCount` _slicingmanager))
  ;[1 1 1] Used so it doesn't reset the food spawn count
  (`GameplayStatics.SpawnSound2D` "/Game/LevelsParameters/InteractFood2.InteractFood2" 1.0 1.0 0.0 null)
  ;[1 1 1] Select cook tool part of the level
  (if (not (> (`/Game/LevelsParameters/SlicingTesting/UnrealExample/SliceGamePawn.CurrentStep` (`self.PawnRef`)) 1))
    (`self.MoveToCookPosition&ClearOthers`)
    (`/Game/LevelsParameters/Cooking/Structures/Cooking_Manager.CheckSelectedCookTool` (`/Game/LevelsParameters/SlicingTesting/UnrealExample/SliceGamePawn.CookingManager` _pawnref_2) _tooltype)
    (if (`|EnumEquality` _tooltype "NewEnumerator1")
      ;;[1 1 1] Skip Adding Water
      (set `/Game/LevelsParameters/SlicingTesting/UnrealExample/SliceGamePawn.CurrentStep` 2 _pawnref)
      ;;[1 1 1] Start slicing part of the level
      (`/Game/LevelsParameters/Cooking/Structures/Cooking_Manager.SwitchToCuttingTable` (`/Game/LevelsParameters/SlicingTesting/UnrealExample/SliceGamePawn.CookingManager` _pawnref) :!label _label)
      (`/Game/LevelsParameters/SlicingTesting/Structures/Slicing_Manager.SpawnLevelFood ` _slicingmanager (- _slicingfoodcount 1))
      (`/Game/LevelsParameters/SlicingTesting/Structures/Slicing_Manager.DecreaseFoodSpawn` _slicingmanager _slicingfoodcount)
      (`self.SetSlicingDialogue`)
      (else
        ;;[1 1 1] Add Water
        (`/Engine/EditorBlueprintResources/StandardMacros.IncrementInt` _currentstep
          (:`  `
            (`self.MoveToFillWater`)
            (if _returnvalue
              (`self.AddWaterHeightPotOrPan` _returnvalue)
              (`KismetSystemLibrary.Delay` 0.3)
              (`SceneComponent.K2_SetRelativeLocation` (`Actor.RootComponent` (`self.PawnRef`)) (560.688248 -45.418207 193.301605) false false)
              (`GameplayStatics.PlaySoundAtLocation` "/Game/LevelsParameters/SlicingTesting/SFX/BoilingWater.BoilingWater" (560.688248 -45.418207 193.301605) (struct) 1.0 1.0 0.0 null null null null)
              (goto _label))))))))

(event `InputTouch`
  (params (Location :type "Vector Structure") (FingerIndex :type "ETouchIndex Enum"))
  ;[1 1 1] Não funciona xD
)

(fn `AddWaterHeightPotOrPan`
  (params (Condition :type Boolean))
  (if Condition
    (if (`|EnumEquality` (`self.ToolType`) "NewEnumerator0")
      (set `self.WaterHeight` 0.8)
      (else
        (set `self.WaterHeight` 0.2)))
    (`NiagaraFunctionLibrary.SpawnSystemAtLocation` "/Game/LevelsParameters/SlicingTesting/VFX/Steam.Steam" (968.2265 202.681345 150.0) (struct) (0.01 0.01 0.01))))

(fn `MoveToCookPosition&ClearOthers`
  (`self.SetPositionCookTool` (`self.ToolType`))
  (bind _outactors (`GameplayStatics.GetAllActorsOfClass` "BP_SelectCookTool_C"))
  (for _array_element _outactors
    (if (not (== _array_element self))
      (`self.K2_DestroyActor` _array_element))))

(fn `MoveToFillWater`
  (bind _output (`|GetArrayItem` (`/Game/LevelsParameters/Cooking/Structures/RecipeDataAsset.RecipeInstructions` (`/Game/LevelsParameters/Cooking/Structures/Cooking_Manager.ActiveCookingFood` (`/Game/LevelsParameters/SlicingTesting/UnrealExample/SliceGamePawn.CookingManager` (`self.PawnRef`)))) 2))
  (bind (_lefts _rights) (`KismetStringLibrary.Split` (`KismetTextLibrary.Conv_TextToString` _output) "("))
  (`SceneComponent.K2_SetRelativeLocation` (`Actor.RootComponent` (`self.PawnRef`)) (679.73545 210.0264 239.414391) false false)
  (bind _foundwidgets (`WidgetBlueprintLibrary.GetAllWidgetsOfClass` "/Game/UIElements/WBP_CommonUI.WBP_CommonUI_C"))
  (set `/Game/UIElements/WBP_CommonUI.RecipeString` (`KismetTextLibrary.Conv_TextToString` _output) (`|GetArrayItem` _foundwidgets))
  (bind _outactors (`GameplayStatics.GetAllActorsOfClass` "/Script/Engine.TextRenderActor"))
  (`TextRenderComponent.K2_SetText` (`TextRenderActor.TextRender` (`|GetArrayItem` _outactors)) (`|FormatText` "{left}\n({right} " _lefts _rights)))

(fn `SetPositionCookTool`
  (params (Selection :type "/Game/LevelsParameters/Cooking/Structures/ECookToolType Enum" :default "NewEnumerator0"))
  (bind _rootcomponent (`self.RootComponent`))
  (switch `/Game/LevelsParameters/Cooking/Structures/ECookToolType` Selection
    (:`NewEnumerator0`
      (`SceneComponent.K2_SetRelativeLocation` _rootcomponent (986.2265 212.681345 112.0) false false))
    (:`NewEnumerator1`
      (`SceneComponent.K2_SetRelativeLocation` _rootcomponent (986.2265 212.681345 92.0) false false))
    (:`NewEnumerator2`
      (`SceneComponent.K2_SetRelativeLocation` _rootcomponent (986.2265 212.681345 98.0) false false))))

(fn `SetSlicingDialogue`
  (bind _output (`|GetArrayItem` (`/Game/LevelsParameters/Cooking/Structures/RecipeDataAsset.RecipeInstructions` (`/Game/LevelsParameters/Cooking/Structures/Cooking_Manager.ActiveCookingFood` (`/Game/LevelsParameters/SlicingTesting/UnrealExample/SliceGamePawn.CookingManager` (`self.PawnRef`)))) 3))
  (bind (_lefts _rights) (`KismetStringLibrary.Split` (`KismetTextLibrary.Conv_TextToString` _output) "that's"))
  (bind (_lefts_2 _rights_2) (`KismetStringLibrary.Split` (`KismetTextLibrary.Conv_TextToString` _output) "comida"))
  (bind _foundwidgets (`WidgetBlueprintLibrary.GetAllWidgetsOfClass` "/Game/UIElements/WBP_CommonUI.WBP_CommonUI_C"))
  (bind _output_2 (`|GetArrayItem` _foundwidgets))
  (set `/Game/UIElements/WBP_CommonUI.DialogueString` "Escolhe a comida que vai trazer mais benefícios para combater o desperdício alimentar" _output_2)
  (`Widget.SetVisibility` (`/Game/UIElements/WBP_CommonUI.VerticalContainer` _output_2) "Visible")
  (set `/Game/UIElements/WBP_CommonUI.RecipeString` (`KismetTextLibrary.Conv_TextToString` _output) _output_2)
  (bind _outactors (`GameplayStatics.GetAllActorsOfClass` "/Script/Engine.TextRenderActor"))
  (bind _asbp_main_game_instance (`/Game/TopDown/Blueprints/CommonFunctionsLibrary.GetGameInstance`))
  (switch `string` (`/Game/TopDown/Blueprints/BP_MainGameInstance.Language` _asbp_main_game_instance)
    (:`pt`
      (bind _textrender (`TextRenderActor.TextRender` (`|GetArrayItem` _outactors)))
      (`TextRenderComponent.K2_SetText` _textrender (`|FormatText` "{left}comida\n{right}" _lefts_2 _rights_2)))
    (:`en`
      (`TextRenderComponent.K2_SetText` _textrender (`|FormatText` "{left}that's\n{right}" _lefts _rights)))))

(fn `SetToolType`
  (switch `string` (`KismetSystemLibrary.GetDisplayName` (`StaticMeshComponent.StaticMesh` (`self.StaticMesh`)))
    (:`Pan`
      (set `self.ToolType` "NewEnumerator2" :!label _label))
    (:`PanWater`
      (goto _label))
    (:`Pot`
      (set `self.ToolType` "NewEnumerator0" :!label _label_2))
    (:`PotWater`
      (goto _label_2))
    (:`Plate`
      (set `self.ToolType` "NewEnumerator1"))))

(fn `UserConstructionScript`
  (`StaticMeshComponent.SetStaticMesh` (`self.StaticMesh`) (`self.ToolMesh`)))